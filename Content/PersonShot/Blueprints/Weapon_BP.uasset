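; Hitscan weapon Blueprint for the player, with magazine and reserve ammo and Fire and Reload events.
; Fire spends a round with a shot sound or dry-fires when empty, then always runs a debug-drawn line trace from Person_Pawn's camera with random spread, leaving the hit unused.
; Reload refills the magazine from the reserve without clamping when the reserve is short.
; The construction script sets ammo and spread defaults.
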(event Custom|Fire
  (CallFunction|AmmoCheck)
  (CallFunction|LineTrace))

(event Custom|Reload
  (bind _ammocount (Variables|Default|GetAmmoCount))
  (if (and (< (Variables|Default|GetCurAmmo) (Variables|Default|GetAmmoCount)) (> (Variables|Default|GetTotalAmmo) 0))
    (Variables|Default|SetTotalAmmo (- (Variables|Default|GetTotalAmmo) (- _ammocount (Variables|Default|GetCurAmmo))))
    (Variables|Default|SetCurAmmo _ammocount)
    (Audio|PlaySoundatLocation "/Game/PersonShot/Audios/Reload_Load.Reload_Load" "0, 0, 0" "0, 0, 0" 1.0 1.0 0.0 0 0 0)))

(fn ConstructionScript
  (Variables|Default|SetAmmoCount 30)
  (Variables|Default|SetTotalAmmo 220)
  (Variables|Default|SetCurAmmo 30)
  (Variables|Default|SetBulletSpread 5e+02))

(fn AmmoCheck
  (bind _curammo (Variables|Default|GetCurAmmo))
  (if (> _curammo 0)
    (Math|Integer|DecrementInt _curammo
      (:%20%20
        (Audio|PlaySoundatLocation "/Game/FirstPerson/Audio/FirstPersonTemplateWeaponFire02.FirstPersonTemplateWeaponFire02" "0, 0, 0" "0, 0, 0" 1.0 1.0 0.0 0 0 0)))
    (else
      (Audio|PlaySoundatLocation "/Game/PersonShot/Audios/DryFire.DryFire" (Math|Vector|MakeVector 0.0 0.0 0.0) "0, 0, 0" 1.0 1.0 0.0 0 0 0))))

(fn LineTrace
  (bind _returnvalue (Game|GetPlayerCharacter 0))
  (bind _bulletspread (Variables|Default|GetBulletSpread))
  (bind _asperson_pawn (Utilities|Casting|CastToPerson_Pawn _returnvalue))
  (bind _personcamera (Variables|/Game/PersonShot/Blueprints/Person_Pawn.Person_Pawn_C|GetPersonCamera _asperson_pawn))
  (bind _returnvalue_2 (Transformation|GetWorldLocation _personcamera))
  (bind _outhit (Collision|LineTraceByChannel _returnvalue_2 (+ _returnvalue_2 (+ (* (Math|Vector|GetForwardVector _personcamera) 2e+04) (Math|Vector|MakeVector (Math|Random|RandomFloatinRange (* _bulletspread -1.0) _bulletspread) (Math|Random|RandomFloatinRange (* _bulletspread -1.0) _bulletspread) (Math|Random|RandomFloatinRange (* _bulletspread -1.0) _bulletspread)))) "TraceTypeQuery1" false 0 "ForDuration")))