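; Grenade actor that explodes on a short fixed fuse after it spawns.
; BeginPlay starts a one-shot timer whose Explosion event spawns a scaled-up Explosion_BP at the mesh location, plays the grenade sound there and destroys the actor.
; The explosion takes its rotation from the CameraBoom of the player character, cast to Person_Pawn, rather than from the grenade itself.
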(event Custom|Explosion
  (bind _staticmesh (Variables|Default|GetStaticMesh))
  (bind _returnvalue (Transformation|GetWorldLocation _staticmesh))
  (Game|SpawnActorfromClass "/Game/PersonShot/Blueprints/Explosion_BP.Explosion_BP_C" (Math|Transform|MakeTransform _returnvalue (Transformation|GetWorldRotation (Variables|/Game/PersonShot/Blueprints/Person_Pawn.Person_Pawn_C|GetCameraBoom (.AsPerson%20Pawn (Utilities|Casting|CastToPerson_Pawn (Game|GetPlayerCharacter 0))))) "3.000000,3.000000,3.000000") "Undefined" 0 0)
  (Audio|PlaySoundatLocation "/Game/PersonShot/Audios/grenade.grenade" _returnvalue "0, 0, 0" 1.0 1.0 0.0 0 0 0)
  (Actor|DestroyActor))

(event EventBeginPlay
  (Utilities|Time|SetTimerbyEvent (delegate Custom|Explosion) 1.2))

(fn ConstructionScript)